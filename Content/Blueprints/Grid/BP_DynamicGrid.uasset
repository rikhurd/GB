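; BP_DynamicGrid is a configurable tile grid actor built procedurally with Geometry Script dynamic meshes.
; The construction script generates line quads through CreateLine, a one-tile selection quad, and floor and tile boxes with simple collision.
; Lines and selection get M_Grid dynamic material instances for color and opacity.
; Helpers convert between tiles and locations, but TileToGridLocation and SetSelectedTile are stubs, and TileValid's bounds checks can never pass.
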(fn `CalculateGridTileLocation`
  (params (TileIndexX :type "Float (double-precision)") (TileIndexY :type "Float (double-precision)"))
  (returns (Location :type "Vector Structure"))
  (bind _tilesize (`self.TileSize`))
  (return (+ (* (`KismetMathLibrary.MakeVector` TileIndexX TileIndexY) _tilesize) (* _tilesize (0.5 0.5 0.0)))))

(fn `CreateLine`
  (params (Start :type "Vector Structure") (End :type "Vector Structure") (Thickness :type "Float (double-precision)") (Vertices :type "Array of Vector Structure") (Triangles :type "Array of IntVector Structure"))
  (locals (HalfThickness :type "Float (double-precision)") (ThicknessDirection :type "Vector Structure" :default (0.0 0.0 0.0)))
  (bind _returnvalue (`KismetArrayLibrary.Array_Length` (`local.Vertices`)))
  (`|ExecutionSequence`
    (:`then_0`
      (set `local.HalfThickness` (/ (`local.Thickness`) 2.0))
      (set `local.ThicknessDirection` (`KismetMathLibrary.Cross_VectorVector` (`KismetMathLibrary.Normal` (- (`local.End`) (`local.Start`))) (0.0 0.0 1.0))))
    (:`then_1`
      (`KismetArrayLibrary.Array_Append` (`local.Triangles`) (`|MakeArray` (make `IntVector` (+ _returnvalue 2) (+ _returnvalue 1) (+ _returnvalue 0)) (make `IntVector` (+ _returnvalue 2) (+ _returnvalue 3) (+ _returnvalue 1))))
      (`KismetArrayLibrary.Array_Append` (`local.Vertices`) (`|MakeArray` (+ (`local.Start`) (* (`local.ThicknessDirection`) (`local.HalfThickness`))) (+ (`local.End`) (* (`local.ThicknessDirection`) (`local.HalfThickness`))) (- (`local.Start`) (* (`local.ThicknessDirection`) (`local.HalfThickness`))) (- (`local.End`) (* (`local.ThicknessDirection`) (`local.HalfThickness`))))))))

(fn `CreateMaterialInstance`
  (params (Color :type "LinearColor Structure") (Opacity :type "Float (double-precision)"))
  (returns (MaterialInstance :type "MaterialInstanceDynamic Object Reference"))
  (locals (DynamicMaterialInstance :type "MaterialInstanceDynamic Object Reference"))
  (bind _returnvalue (`KismetMaterialLibrary.CreateDynamicMaterialInstance` "/Game/Materials/M_Grid.M_Grid"))
  (bind _output_get (set `local.DynamicMaterialInstance` _returnvalue))
  (`MaterialInstanceDynamic.SetVectorParameterValue` _output_get "Color" (`local.Color`))
  (`MaterialInstanceDynamic.SetScalarParameterValue` (`local.DynamicMaterialInstance`) "Opacity" (`local.Opacity`))
  (return (`local.DynamicMaterialInstance`)))

(fn `CreateMeshSection`
  (params (TargetMesh :type "DynamicMesh Object Reference") (VerticesArray :type "Array of Vector Structure (by ref)") (TrianglesArray :type "Array of IntVector Structure (by ref)"))
  (`|ExecutionSequence`
    (:`then_0`
      (bind _vectorlist (`GeometryScriptLibrary_ListUtilityFunctions.ConvertArrayToVectorList` VerticesArray))
      (`GeometryScriptLibrary_MeshBasicEditFunctions.AddVerticesToMesh` TargetMesh _vectorlist))
    (:`then_1`
      (bind _trianglelist (`GeometryScriptLibrary_ListUtilityFunctions.ConvertArrayToTriangleList` TrianglesArray))
      (`GeometryScriptLibrary_MeshBasicEditFunctions.AddTrianglesToMesh` TargetMesh _trianglelist 0 false null))))

(fn `GetNewDynamicMesh`
  (params (DynamicMeshComponent :type "BaseDynamicMeshComponent Object Reference"))
  (returns (DynamicMesh :type "DynamicMesh Object Reference"))
  (bind _returnvalue (`BaseDynamicMeshComponent.GetDynamicMesh` DynamicMeshComponent))
  (bind _returnvalue_2 (`DynamicMesh.Reset` _returnvalue))
  (return _returnvalue_2))

(fn `GridHeight`
  (returns (ReturnValue :type "Float (double-precision)"))
  (bind _gridsize_x (break `IntPoint` (`self.GridSize`)))
  (return (* _gridsize_x (`self.TileSize`))))

(fn `GridWidth`
  (returns (ReturnValue :type "Float (double-precision)"))
  (bind (_gridsize_x _gridsize_y) (break `IntPoint` (`self.GridSize`)))
  (return (* _gridsize_y (`self.TileSize`))))

(fn `LocationToTile`
  (params (Location :type "Vector Structure"))
  (returns (Valid :type Boolean) (Row :type Integer) (Column :type Integer))
  (bind (_returnvalue_x _returnvalue_y) (`KismetMathLibrary.BreakVector` (`self.K2_GetActorLocation`)))
  (bind _returnvalue_x_2 (`KismetMathLibrary.BreakVector` (`self.K2_GetActorLocation`)))
  (bind (_gridsize_x _gridsize_y) (break `IntPoint` (`self.GridSize`)))
  (bind (_location_x _location_y) (`KismetMathLibrary.BreakVector` (`local.Location`)))
  (bind _gridsize_x_2 (break `IntPoint` (`self.GridSize`)))
  (bind _location_x_2 (`KismetMathLibrary.BreakVector` (`local.Location`)))
  (bind _returnvalue (`KismetMathLibrary.FFloor` (* (/ (- _location_y _returnvalue_y) (`self.GridHeight`)) _gridsize_y)))
  (bind _returnvalue_2 (`KismetMathLibrary.FFloor` (* (/ (- _location_x_2 _returnvalue_x_2) (`self.GridWidth`)) _gridsize_x_2)))
  (bind _valid (`self.TileValid` _returnvalue_2 _returnvalue)
    (:`Execute2`
      (return _valid _returnvalue_2 _returnvalue))))

(fn `SetSelectedTile`
  (params (Row :type Integer) (Column :type Integer)))

(fn `TileToGridLocation`
  (params (Row :type Integer) (Column :type Integer) (Center :type Boolean))
  (returns (Valid :type Boolean) (GridLocation :type "Vector2D Structure"))
  (return false (0.0 0.0)))

(fn `UserConstructionScript`
  (locals (LineMaterialInstance :type "MaterialInstanceDynamic Object Reference") (SelectionMaterialInstance :type "MaterialInstanceDynamic Object Reference") (LineStart :type "Float (double-precision)") (LineEnd :type "Float (double-precision)") (LineVertices :type "Array of Vector Structure") (SelectionVertices :type "Array of Vector Structure") (LineTriangles :type "Array of IntVector Structure") (SelectionTriangles :type "Array of IntVector Structure"))
  (bind _linestart (`local.LineStart`))
  (bind (_gridsize_x _gridsize_y) (break `IntPoint` (`self.GridSize`)))
  (bind (_gridsize_x_2 _gridsize_y_2) (break `IntPoint` (`self.GridSize`)))
  (bind _tilesize (`self.TileSize`))
  (bind _gridsize_x_3 (break `IntPoint` (`self.GridSize`)))
  (bind (_gridsize_x_4 _gridsize_y_3) (break `IntPoint` (`self.GridSize`)))
  (bind _linestart_2 (`local.LineStart`))
  (bind _returnvalue (/ _tilesize 2.0))
  (bind _returnvalue_2 (* (`KismetMathLibrary.Conv_IntToDouble` _gridsize_y) (`self.TileSize`)))
  (bind _returnvalue_3 (* (`KismetMathLibrary.Conv_IntToDouble` _gridsize_x) (`self.TileSize`)))
  (bind _returnvalue_4 (* (`KismetMathLibrary.Conv_IntToDouble` _gridsize_x_2) (`self.TileSize`)))
  (bind _returnvalue_5 (* (`KismetMathLibrary.Conv_IntToDouble` _gridsize_y_2) (`self.TileSize`)))
  (bind (_returnvalue_x _returnvalue_y) (`KismetMathLibrary.BreakVector` (/ (`KismetMathLibrary.MakeVector` _returnvalue_3 _returnvalue_2) 2.0)))
  (bind _materialinstance (`self.CreateMaterialInstance` (`self.LineColor`) (`self.LineOpcaity`)))
  (set `local.LineMaterialInstance` _materialinstance)
  (bind _materialinstance_2 (`self.CreateMaterialInstance` (`self.SelectionColor`) (`self.SelectionOpacity`)))
  (set `local.SelectionMaterialInstance` _materialinstance_2)
  (bind _dynamicmesh (`self.GetNewDynamicMesh` (`self.DynamicMeshComponent`)))
  (bind _dynamicmesh_2 (`self.GetNewDynamicMesh` (`self.GridSelectionMesh`)))
  (bind _dynamicmesh_3 (`self.GetNewDynamicMesh` (`self.GridFloorMesh`)))
  (bind _dynamicmesh_4 (`self.GetNewDynamicMesh` (`self.GridTileMesh`)))
  (`|ExecutionSequence`
    (:`then_0`
      (for _index (range (+ _gridsize_x_3 1))
        (set `local.LineStart` (* _index (`self.TileSize`)))
        (set `local.LineEnd` (`self.GridWidth`))
        (`self.CreateLine` (`KismetMathLibrary.MakeVector` _linestart) (`KismetMathLibrary.MakeVector` _linestart (`local.LineEnd`)) (`self.LineThickness`) (`local.LineVertices`) (`local.LineTriangles`))))
    (:`then_1`
      (for _index_2 (range (+ _gridsize_y_3 1))
        (set `local.LineStart` (* _index_2 (`self.TileSize`)))
        (set `local.LineEnd` (`self.GridHeight`))
        (`self.CreateLine` (`KismetMathLibrary.MakeVector` 0.0 _linestart_2) (`KismetMathLibrary.MakeVector` (`local.LineEnd`) _linestart_2) (`self.LineThickness`) (`local.LineVertices`) (`local.LineTriangles`))))
    (:`then_2`
      (`self.CreateMeshSection` _dynamicmesh (`local.LineVertices`) (`local.LineTriangles`))
      (`PrimitiveComponent.SetMaterial` (`self.DynamicMeshComponent`) 0 (`local.LineMaterialInstance`)))
    (:`then_3`
      (`self.CreateLine` (`KismetMathLibrary.MakeVector` 0.0 _returnvalue) (`KismetMathLibrary.MakeVector` _tilesize _returnvalue) _tilesize (`local.SelectionVertices`) (`local.SelectionTriangles`))
      (`self.CreateMeshSection` _dynamicmesh_2 (`local.SelectionVertices`) (`local.SelectionTriangles`))
      (`PrimitiveComponent.SetMaterial` (`self.GridSelectionMesh`) 0 (`local.SelectionMaterialInstance`)))
    (:`then_4`
      ; Grid Floor mesh
      (bind _simplecollision (`GeometryScriptLibrary_MeshPrimitiveFunctions.AppendBoxWithCollision` _dynamicmesh_3 (struct) (`KismetMathLibrary.MakeTransform` (/ (`KismetMathLibrary.MakeVector` _returnvalue_4 _returnvalue_5) 2.0)) _returnvalue_4 _returnvalue_5 100.0 0 0 0 "Base" null))
      (`GeometryScriptLibrary_CollisionFunctions.SetSimpleCollisionOfDynamicMeshComponent` _simplecollision (`self.GridFloorMesh`) (struct) null))
    (:`then_5`
      ; Grid Tile mesh
      (bind _simplecollision_2 (`GeometryScriptLibrary_MeshPrimitiveFunctions.AppendBoxWithCollision` _dynamicmesh_4 (struct) (`KismetMathLibrary.MakeTransform` (`KismetMathLibrary.MakeVector` _returnvalue_x _returnvalue_y (`self.GridFloorMeshOffset`))) _returnvalue_3 _returnvalue_2 (`self.GridFloorMeshHeight`) 0 0 0 "Base" null))
      (`GeometryScriptLibrary_CollisionFunctions.SetSimpleCollisionOfDynamicMeshComponent` _simplecollision_2 (`self.GridTileMesh`) (struct) null))))